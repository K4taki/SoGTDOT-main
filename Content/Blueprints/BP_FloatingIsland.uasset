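; BP_FloatingIsland is a floating island whose static mesh moves back and forth endlessly between a start point and an end point component.
; After a short delay at BeginPlay, two timelines alternately lerp the mesh's world location between Startpunkt and Endpunkt, one for each direction.
; Each timeline waits at its destination before calling the opposite event, forming a continuous ping-pong loop.
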(event Custom|CustomEvent_0
  ;[0.5011 0.06198 1] Insel Floating
  (bind _alpha (Timeline|Alpha%20lerp%20timer PlayFromStart)
    (:Update
      (Transformation|SetWorldLocation (Variables|Default|GetStaticMesh) (Math|Vector|Lerp(Vector) (Transformation|GetWorldLocation (Variables|Default|GetStartpunkt)) (Transformation|GetWorldLocation (Variables|Default|GetEndpunkt)) _alpha) false false))
    (:Finished
      (Utilities|FlowControl|Delay 3.0)
      (CallFunction|FromEndtoStart))))

(event Custom|From%20End%20to%20Start
  ;[0.5011 0.06198 1] Insel Floating
  (bind _alpha (Timeline|Timeline_0 PlayFromStart)
    (:Update
      (Transformation|SetWorldLocation (Variables|Default|GetStaticMesh) (Math|Vector|Lerp(Vector) (Transformation|GetWorldLocation (Variables|Default|GetEndpunkt)) (Transformation|GetWorldLocation (Variables|Default|GetStartpunkt)) _alpha) false false))
    (:Finished
      (Utilities|FlowControl|Delay 3.0)
      (CallFunction|CustomEvent0))))

(event EventBeginPlay
  ;[0.5011 0.06198 1] Insel Floating
  (Utilities|FlowControl|Delay 3.0)
  (CallFunction|CustomEvent0))

(fn ConstructionScript)