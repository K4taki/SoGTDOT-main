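; BP_Kiste is a crate that drops or tumbles after the player touches it, then respawns at its starting location.
; An overlap of its Box by BP_Spieler waits a configurable delay, then enables physics simulation on the static mesh.
; Five seconds later it spawns a fresh BP_Kiste at the location saved on BeginPlay, passing on the same delay, and destroys itself.
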(event OnComponentBeginOverlap(Box)
  (params (OverlappedComponent :type Primitive%20Component%20Object%20Reference) (OtherActor :type Actor%20Object%20Reference) (OtherComp :type Primitive%20Component%20Object%20Reference) (OtherBodyIndex :type Integer) (bFromSweep :type Boolean) (SweepResult :type Hit%20Result%20Structure%20%28by%20ref%29))
  (Utilities|Casting|CastToBP_Spieler OtherActor)
  (Utilities|FlowControl|Delay (Variables|Default|GetDelay))
  (Physics|SetSimulatePhysics (Variables|Default|GetStaticMesh) true)
  (Utilities|FlowControl|Delay 5.0)
  (Game|SpawnActorfromClass "BP_Kiste_C" (Math|Transform|MakeTransform (Variables|Default|GetStart) "0, 0, 0" "1,1,1") "Undefined" 0 (Variables|Default|GetDelay) 0)
  (Actor|DestroyActor))

(event EventBeginPlay
  (Variables|Default|SetStart (Transformation|GetActorLocation)))

(fn ConstructionScript)